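; EndGameVolume is a volume that signals the end of the game once all bots that started inside it are dead.
; BeginPlay stores the Bot actors overlapping Box1 in the Bots array.
; Each Tick removes at most one bot with HitPoints below 1, then fires the OnEndGame dispatcher once when the array is empty, including when no bots were found.
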(event `self.ReceiveBeginPlay`
  ;[1 1 1] BeginPlay. Gather all bots inside this volume and store them into array
  (`KismetArrayLibrary.Array_Clear` (`self.Bots`))
  (bind _outactors (`KismetSystemLibrary.ComponentOverlapActors_NEW` (`self.Box1`) (`self.GetTransform`) (`self.NewVar`) "/Game/Blueprints/Bot.Bot_C"))
  (for _array_element _outactors
    (bind _asbot (cast `/Game/Blueprints/Bot` _array_element))
    (`KismetArrayLibrary.Array_Add` (`self.Bots`) _asbot)))

(event `self.ReceiveTick`
  (params (DeltaSeconds :type "Float (single-precision)"))
  (bind _bots (`self.Bots`))
  ;[1 1 1] Tick. Check if all bots in 'Bots' array are dead, if so, call EndGame event (most likely it will be bound inside level blueprint
  (for _array_element _bots
    (if (< (`/Game/Blueprints/Bot.HitPoints` _array_element) 1)
      (set `self.temp` _array_element)
      (break)))
  (`KismetArrayLibrary.Array_RemoveItem` _bots (`self.temp`))
  (if (== (`KismetArrayLibrary.Array_Length` _bots) 0)
    (`/Engine/EditorBlueprintResources/StandardMacros.DoOnce` false
      (:`Completed`
        (`self.CallOnEndGame`)))))

(fn `UserConstructionScript`)