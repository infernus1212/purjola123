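; UCShell is a bouncing shell, likely an ejected casing, with rotation and movement components.
; Hits on anything except a Bot increment a bounce counter and play a random clip from an audio array; SoundPlayed never latches.
; Near MaxBounce, it zeroes rotation rate and velocity and levels its pitch.
; Tick matches playing audio's pitch to global time dilation, so sound follows slow motion.
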(event `self.ReceiveTick`
  (params (DeltaSeconds :type "Float (single-precision)"))
  (bind _audiocomponent (`self.AudioComponent`))
  (if (`AudioComponent.IsPlaying` _audiocomponent)
    (`AudioComponent.SetPitchMultiplier` _audiocomponent (`GameplayStatics.GetGlobalTimeDilation`))))

(event `self.ReceiveHit`
  (params (MyComp :type "PrimitiveComponent Object Reference") (Other :type "Actor Object Reference") (OtherComp :type "PrimitiveComponent Object Reference") (bSelfMoved :type Boolean) (HitLocation :type "Vector Structure") (HitNormal :type "Vector Structure") (NormalImpulse :type "Vector Structure") (Hit :type "HitResult Structure (by ref)"))
  (bind _audiocomponent (`self.AudioComponent`))
  (bind _audioarray (`self.AudioArray`))
  (bind _returnvalue (+ (`self.BounceCounter`) 1))
  ;[1 1 1] Make sure we bounce from bot
  (cast `/Game/Blueprints/Bot` Other
    (:`then`
      (if (not true)
        (set `self.BounceCounter` _returnvalue :!label _label)
        (if (not (`self.bSoundPlayed`))
          ;[1 1 1] Play random shell audio from array
          (`AudioComponent.SetSound` _audiocomponent (`KismetArrayLibrary.Array_Get` _audioarray (`KismetMathLibrary.RandomIntegerInRange` 0 (- (`KismetArrayLibrary.Array_Length` _audioarray) 1))))
          (`AudioComponent.Play` _audiocomponent 0.0)
          (set `AudioComponent.VolumeMultiplier` 0.2 _audiocomponent)
          (set `self.bSoundPlayed` false))
        (if (>= _returnvalue (`self.MaxBounce`))
          (set `RotatingMovementComponent.RotationRate` (struct) (`self.ShellRotationComponent`))
          (set `MovementComponent.Velocity` (0.0 0.0 0.0) (`self.ShellMovementComponent`))
          (`self.K2_SetActorRotation` (`KismetMathLibrary.MakeRotator` (.roll (`self.K2_GetActorRotation`)) 0.0 (.yaw (`self.K2_GetActorRotation`)))))))
    (:`CastFailed`
      (goto _label))))

(fn `UserConstructionScript`)