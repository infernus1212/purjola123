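; Enemy bot gun weapon Blueprint that fires projectiles at a target with random aim scatter and tracks ammo up to a maximum.
; BotShot spawns a muzzle effect, a projectile aimed from the Projectile socket that ignores its owner, a red beam trail, fire audio, and an ejected shell with randomized velocity and spin.
; Construction brightens the mesh's second material through a dynamic instance and lowers the action audio volume.
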(event `self.ReceiveTick`
  (params (DeltaSeconds :type "Float (single-precision)"))
  (`parent.ReceiveTick` DeltaSeconds))

(fn `Add Ammo`
  (returns (NewParam :type Boolean))
  (locals (bAdded :type Boolean))
  (bind _returnvalue (+ (`self.Ammo`) 1))
  (if (<= _returnvalue (`self.MaxAmmo`))
    (set `self.Ammo` _returnvalue)
    (set `local.bAdded` true)
    (else
      (set `local.bAdded` false)))
  (return (`local.bAdded`)))

(fn `BotShot`
  (params (inTarget :type "Actor Object Reference") (inEnemyOwner :type "/Game/Blueprints/Enemy Object Reference"))
  (bind _returnvalue (`SceneComponent.GetSocketLocation` (`self.SkeletalMeshComponent`) "Projectile"))
  (bind _returnvalue_2 (`GameplayStatics.SpawnEmitterAtLocation` "/Game/StarterContent/Particles/P_Explosion.P_Explosion" _returnvalue))
  (`SceneComponent.SetRelativeScale3D` _returnvalue_2 (0.1 0.1 0.1))
  (bind _returnvalue_3 (`|SpawnActorFromClass` "/Game/Blueprints/UCProjectile.UCProjectile_C" (`KismetMathLibrary.MakeTransform` _returnvalue (`KismetMathLibrary.FindLookAtRotation` _returnvalue (+ (`self.K2_GetActorLocation` inTarget) (* (`KismetMathLibrary.RandomUnitVector`) (`self.RandomAimOffset`))))) "AlwaysSpawn" "OverrideRootScale"))
  (bind _collisioncomponent (`/Game/Blueprints/UCProjectile.CollisionComponent` _returnvalue_3))
  ;[1 1 1] Disable self hit
  (`PrimitiveComponent.IgnoreActorWhenMoving` _collisioncomponent inEnemyOwner true)
  (`AudioComponent.Play` (`self.BaseActionAudioComp`) 0.0)
  (bind _returnvalue_4 (`GameplayStatics.SpawnEmitterAttached` "/Game/Particles/BeamParticle.BeamParticle" _collisioncomponent))
  (`ParticleSystemComponent.SetVectorParameter` _returnvalue_4 "InitialColor" (50.0 1.0 1.0))
  (`ParticleSystemComponent.SetBeamTargetPoint` _returnvalue_4 0 _returnvalue 0)
  ;[1 1 1] Spawn shell
  (bind _returnvalue_5 (`|SpawnActorFromClass` "/Game/Blueprints/UCShell.UCShell_C" (`KismetMathLibrary.MakeTransform` (`self.K2_GetActorLocation`) (`self.K2_GetActorRotation`) (0.2 0.2 0.2)) "AlwaysSpawn" "OverrideRootScale"))
  (set `MovementComponent.Velocity` (+ (* (`KismetMathLibrary.GetUpVector` (struct)) (+ (`self.UpShellVelocityMultiplier`) (`KismetMathLibrary.RandomFloatInRange` -100.0 100.0))) (* (`KismetMathLibrary.GetRightVector` (`self.K2_GetActorRotation`)) (+ (`self.RightShellVelocityMultiplier`) (`KismetMathLibrary.RandomFloatInRange` -100.0 100.0))) (* (`KismetMathLibrary.GetForwardVector` (`self.K2_GetActorRotation`)) (`KismetMathLibrary.RandomFloatInRange` -50.0 50.0))) (`/Game/Blueprints/UCShell.ShellMovementComponent` _returnvalue_5))
  (set `RotatingMovementComponent.RotationRate` (* (`KismetMathLibrary.RandomRotator` false) 3.0) (`/Game/Blueprints/UCShell.ShellRotationComponent` _returnvalue_5)))

(fn `UserConstructionScript`
  (bind _skeletalmeshcomponent (`self.SkeletalMeshComponent`))
  (`parent.UserConstructionScript`)
  (bind _returnvalue (`PrimitiveComponent.CreateDynamicMaterialInstance` _skeletalmeshcomponent 1 "/Game/Materials/M_TestMat.M_TestMat"))
  (bind _returnvalue_2 (`MaterialInstanceDynamic.K2_GetVectorParameterValue` _returnvalue "BaseColor"))
  (`MaterialInstanceDynamic.SetVectorParameterValue` _returnvalue "BaseColor" (* _returnvalue_2 2.0))
  (`PrimitiveComponent.SetMaterial` _skeletalmeshcomponent 1 _returnvalue)
  (`AudioComponent.SetVolumeMultiplier` (`self.BaseActionAudioComp`) 0.2))