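; Level actor that tracks the best completion time for a level and shows it on the HUD.
; On BeginPlay it enables the HUD's high score display and loads a HighScoreSave from its slot, or creates one with a default record.
; CheckForLevelRecord stops the character's timer and stores the elapsed time in the game instance's LevelTimes by level index.
; A faster time overwrites the record, saves it to the slot and updates the HUD.
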(event `self.ReceiveBeginPlay`
  ;[1 1 1] BeginPlay and Initialize variables. Tell HUD to actually draw timer and load best score for this level
  (bind _asmy_hud (cast `/Game/Blueprints/MyHUD` (`PlayerController.GetHUD` (`GameplayStatics.GetPlayerController` 0))))
  (set `/Game/Blueprints/MyHUD.bDrawHighScore` true _asmy_hud)
  (bind _returnvalue (`GameplayStatics.DoesSaveGameExist` (`KismetStringLibrary.Conv_NameToString` (`self.SaveSlotName`))))
  (if _returnvalue
    (bind _returnvalue_2 (`GameplayStatics.LoadGameFromSlot` (`KismetStringLibrary.Conv_NameToString` (`self.SaveSlotName`))))
    (bind _ashigh_score_save (cast `/Game/Blueprints/HighScoreSave` _returnvalue_2))
    (set `self.HighScoreObject` _ashigh_score_save)
    (else
      (bind _returnvalue_3 (`GameplayStatics.CreateSaveGameObject` "/Game/Blueprints/HighScoreSave.HighScoreSave_C"))
      (bind _ashigh_score_save_2 (cast `/Game/Blueprints/HighScoreSave` _returnvalue_3))
      (set `self.HighScoreObject` _ashigh_score_save_2)
      (set `/Game/Blueprints/HighScoreSave.HighScore` (`self.DefaultHighScore`) (`self.HighScoreObject`))))
  (bind _asmy_hud_2 (cast `/Game/Blueprints/MyHUD` (`PlayerController.GetHUD` (`GameplayStatics.GetPlayerController` 0))))
  (set `/Game/Blueprints/MyHUD.CurrentHighScore` (`/Game/Blueprints/HighScoreSave.HighScore` (`self.HighScoreObject`)) _asmy_hud_2))

(event `CheckForLevelRecord`
  (bind _highscoreobject (`self.HighScoreObject`))
  ;[1 1 1] Should be called when player has completed the level and you want to stop timer and check if the record was beaten.
  (bind _asmy_character (cast `/Game/Blueprints/MyCharacter` (`GameplayStatics.GetPlayerCharacter` 0)))
  (set `/Game/Blueprints/MyCharacter.bUseTimer` false _asmy_character)
  (bind _asucgame_instance (cast `/Game/Blueprints/UCGameInstance` (`GameplayStatics.GetGameInstance`)))
  (bind _elapsedleveltime (`/Game/Blueprints/MyCharacter.ElapsedLevelTime` _asmy_character))
  (`KismetArrayLibrary.Array_Set` (`/Game/Blueprints/UCGameInstance.LevelTimes` _asucgame_instance) (`self.LevelIndex`) _elapsedleveltime)
  (if (< _elapsedleveltime (`/Game/Blueprints/HighScoreSave.HighScore` _highscoreobject))
    (set `/Game/Blueprints/HighScoreSave.HighScore` _elapsedleveltime _highscoreobject)
    (`GameplayStatics.SaveGameToSlot` (`self.HighScoreObject`) (`KismetStringLibrary.Conv_NameToString` (`self.SaveSlotName`)))
    (bind _asmy_hud (cast `/Game/Blueprints/MyHUD` (`PlayerController.GetHUD` (`GameplayStatics.GetPlayerController` 0))))
    (set `/Game/Blueprints/MyHUD.CurrentHighScore` (`/Game/Blueprints/HighScoreSave.HighScore` (`self.HighScoreObject`)) _asmy_hud)))

(fn `UserConstructionScript`)