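; Knife weapon that detects stab hits by line tracing between its blade sockets every tick while the base action montage plays on the parent skeletal mesh.
; Hit Enemy or Bot actors get OnStabbed and a body hit sound.
; Both casts run in sequence, and each failure plays the wall sound, pushes simulating physics components and damages destructible ones.
; Hit audio pitch follows global time dilation.
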(event `self.ReceiveTick`
  (params (DeltaSeconds :type "Float (single-precision)"))
  (bind _skeletalmeshcomponent (`self.SkeletalMeshComponent`))
  (bind _returnvalue (`SceneComponent.GetSocketLocation` _skeletalmeshcomponent "BladeBottom"))
  (`parent.ReceiveTick` DeltaSeconds)
  (`|ExecutionSequence`
    (:`then_0`
      ;[1 1 1] Slow Audio
      (`AudioComponent.SetPitchMultiplier` (`self.WallHitAudioComp`) (`GameplayStatics.GetGlobalTimeDilation`))
      (`AudioComponent.SetPitchMultiplier` (`self.BotHitAudioComp`) (`GameplayStatics.GetGlobalTimeDilation`)))
    (:`then_1`
      ;[1 1 1] Check if we're stabbing
      (bind _asskeletal_mesh_component (cast `SkeletalMeshComponent` (`SceneComponent.GetAttachParent` (`self.SkeletalMeshComponent`))))
      (if (`AnimInstance.Montage_IsPlaying` (`SkeletalMeshComponent.GetAnimInstance` _asskeletal_mesh_component) (`self.BaseActionMontage`))
        ;[1 1 1] Do stab trace!
        (bind (_outhit _returnvalue_2) (`KismetSystemLibrary.LineTraceSingle` (`SceneComponent.GetSocketLocation` _skeletalmeshcomponent "BladeTop") _returnvalue "TraceTypeQuery1"))
        (if _returnvalue_2
          (set `self.bPerformingStab` true)
          (`|ExecutionSequence`
            (:`then_0`
              (bind (_bblockinghit _binitialoverlap _time _location _impactpoint _normal _impactnormal _physmat _hitactor _hitcomponent _hitbonename) (`GameplayStatics.BreakHitResult` _outhit))
              (bind _asenemy (cast `/Game/Blueprints/Enemy` _hitactor)
                (:`then`
                  (`/Game/Blueprints/Enemy.OnStabbed` _asenemy _impactpoint _impactnormal _hitbonename)
                  (`AudioComponent.Play` (`self.BotHitAudioComp`) 0.0 :!label _label))
                (:`CastFailed`
                  (`AudioComponent.Play` (`self.WallHitAudioComp`) 0.0 :!label _label_2)
                  (if (`SceneComponent.IsSimulatingPhysics` _hitcomponent "None")
                    (bind _returnvalue_3 (`KismetMathLibrary.Normal` (- _impactpoint _returnvalue)))
                    (`PrimitiveComponent.AddImpulseAtLocation` _hitcomponent (* _returnvalue_3 (`self.StabImpulse`)) _impactpoint "None")
                    (bind _asdestructible_component (cast `DestructibleComponent` _hitcomponent))
                    (`DestructibleComponent.ApplyDamage` _asdestructible_component (`self.StabDamage`) _impactpoint _returnvalue_3 (`self.StabImpulse`))))))
            (:`then_1`
              (bind _asbot (cast `/Game/Blueprints/Bot` _hitactor)
                (:`then`
                  (`/Game/Blueprints/Bot.OnStabbed` _asbot _impactpoint _impactnormal _hitbonename)
                  (goto _label))
                (:`CastFailed`
                  (goto _label_2))))))
        (else
          (set `self.bPerformingStab` false))))))

(fn `UserConstructionScript`
  (`parent.UserConstructionScript`))