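; A glass volume that refills the player's gun with a limited number of ammo pickups and overrides game speed while the player is inside.
; Inside, standing still eases global time dilation to normal and moving eases it to slow motion, with the player's custom time compensated and mid-transition reversals resuming from the current speed.
; Ammo arrives on a dilation-corrected timer, counted down on camera-facing text.
; Exit or depletion returns speed control to MyCharacter; depletion also shrinks, fades and destroys the volume.
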(event `self.Volume.OnComponentBeginOverlap`
  (params (OverlappedComponent :type "PrimitiveComponent Object Reference") (OtherActor :type "Actor Object Reference") (OtherComp :type "PrimitiveComponent Object Reference") (OtherBodyIndex :type Integer) (bFromSweep :type Boolean) (SweepResult :type "HitResult Structure (by ref)"))
  ;[1 1 1] On enter event
  (if (not (`self.bDestroy`))
    (bind _asmy_character (cast `/Game/Blueprints/MyCharacter` OtherActor))
    (set `/Game/Blueprints/MyCharacter.InVolume` true _asmy_character)
    (set `self.CharInVolume` true)
    (set `self.Alpha` 0.0)
    (set `self.Transition From` (`/Game/Blueprints/MyCharacter.SlomoTime` _asmy_character))
    (set `self.bTransitionCompleted` false)
    (set `self.CalcAlphaTime` true)
    (set `self.Last Slomo Value` (`GameplayStatics.GetGlobalTimeDilation`))
    (set `self.State` false)))

(event `self.Volume.OnComponentEndOverlap`
  (params (OverlappedComponent :type "PrimitiveComponent Object Reference") (OtherActor :type "Actor Object Reference") (OtherComp :type "PrimitiveComponent Object Reference") (OtherBodyIndex :type Integer))
  ;[1 1 1] On leave event
  (if (not (`self.bDestroy`))
    (bind _asmy_character (cast `/Game/Blueprints/MyCharacter` OtherActor))
    (set `/Game/Blueprints/MyCharacter.InVolume` false _asmy_character)
    (set `self.CharInVolume` false)
    (`/Game/Blueprints/MyCharacter.Open SlomoIn Gate` _asmy_character)
    (set `/Game/Blueprints/MyCharacter.Last SlomoOut Value` (`GameplayStatics.GetGlobalTimeDilation`) _asmy_character)
    (set `/Game/Blueprints/MyCharacter.CalcSlomoInAlpha` true _asmy_character)
    (set `self.ActionTimer` 0.0)))

(event `self.ReceiveTick`
  (params (DeltaSeconds :type "Float (single-precision)"))
  (bind _returnvalue (`GameplayStatics.GetGlobalTimeDilation`))
  (bind _returnvalue_2 (`GameplayStatics.GetPlayerCharacter` 0))
  (bind _actioncounter (`self.ActionCounter`))
  (bind _state (`self.State`))
  (bind _textrender1 (`self.TextRender1`))
  (`|ExecutionSequence`
    (:`then_0`
      (if (and (`self.CharInVolume`) (not (`self.bDestroy`)))
        (`|ExecutionSequence`
          (:`then_0`
            (if (== (`self.GetVelocity` (`GameplayStatics.GetPlayerCharacter` 0)) (0.0 0.0 0.0) :`ErrorTolerance` 0.0)
              ;[1 1 1] Set player state (in transistion to new game speed or not)
              (set `self.TransitionTo` (`self.NormalTime`))
              (if (not _state)
                (set `self.State` true)
                (set `self.Transition From` (`self.SlomoTime`))
                (set `self.Alpha` 0.0 :!label _label)
                (set `self.bTransitionCompleted` false)
                (set `self.CalcAlphaTime` true)
                (set `self.Last Slomo Value` (`GameplayStatics.GetGlobalTimeDilation`)))
              (else
                (set `self.TransitionTo` (`self.SlomoTime`))
                (if _state
                  (set `self.State` false)
                  (set `self.Transition From` (`self.NormalTime`))
                  (goto _label)))))
          (:`then_1`
            (if (not (`self.bTransitionCompleted`))
              ;[1 1 1] Transition function
              (bind (_time _alpha) (`self.Transition` DeltaSeconds (`self.Transition From`) (`self.TransitionTo`) (`self.Alpha`) (`self.TransitionTime`)))
              (`GameplayStatics.SetGlobalTimeDilation` _time)
              (set `self.Alpha` _alpha)
              (bind _asmy_character (cast `/Game/Blueprints/MyCharacter` (`GameplayStatics.GetPlayerCharacter` 0)))
              (`/Game/Blueprints/MyCharacter.CustomTime` _asmy_character (/ 1.0 _time))
              (`/Game/Blueprints/MyCharacter.Change PostProcess` _asmy_character)))
          (:`then_2`
            (if (< (`self.ActionCounter`) (`self.NumberOfActions`))
              ;[1 1 1] Add bullets function and interval timer
              (set `self.ActionTimer` (+ (/ DeltaSeconds (`GameplayStatics.GetGlobalTimeDilation`)) (`self.ActionTimer`)))
              (if (>= (`self.ActionTimer`) (`self.ActionInterval`))
                (bind _asmy_character_2 (cast `/Game/Blueprints/MyCharacter` _returnvalue_2))
                (bind _bool (`/Game/Blueprints/MyCharacter.AddAmmoToGun` _asmy_character_2))
                (if _bool
                  (set `self.ActionCounter` (+ _actioncounter 1))
                  (set `self.ActionTimer` 0.0)
                  (`TextRenderComponent.K2_SetText` (`self.TextRender1`) (`KismetTextLibrary.Conv_StringToText` (`KismetStringLibrary.Conv_IntToString` (- (`self.NumberOfActions`) _actioncounter))))
                  (else
                    (set `self.ActionTimer` 0.0))))
              (else
                ;[1 1 1] Bullets depleted, destroy volume,  change game speed
                (bind _asmy_character_3 (cast `/Game/Blueprints/MyCharacter` _returnvalue_2))
                (set `/Game/Blueprints/MyCharacter.InVolume` false _asmy_character_3)
                (if (== (`self.GetVelocity` _asmy_character_3) (0.0 0.0 0.0) :`ErrorTolerance` 0.0)
                  (`/Game/Blueprints/MyCharacter.Open SlomoOut Gate` _asmy_character_3)
                  (set `/Game/Blueprints/MyCharacter.CalcSlomoOutAlpha` true _asmy_character_3)
                  (set `/Game/Blueprints/MyCharacter.Last SlomoIn Value` _returnvalue _asmy_character_3)
                  (else
                    (`/Game/Blueprints/MyCharacter.Open SlomoIn Gate` _asmy_character_3)
                    (set `/Game/Blueprints/MyCharacter.CalcSlomoInAlpha` true _asmy_character_3)
                    (set `/Game/Blueprints/MyCharacter.Last SlomoOut Value` _returnvalue _asmy_character_3)))
                (set `self.bDestroy` true)
                (`self.onDestroy`)))))))
    (:`then_1`
      ;[1 1 1] Rotate text to always face player
      (`SceneComponent.K2_SetWorldRotation` _textrender1 (`KismetMathLibrary.MakeRotator` 0.0 0.0 (+ (.yaw (`KismetMathLibrary.MakeRotFromX` (- (`SceneComponent.K2_GetComponentLocation` _textrender1) (`self.K2_GetActorLocation` (`GameplayStatics.GetPlayerCameraManager` 0))))) 180.0)) false false))))

(event `onDestroy`
  ;[1 1 1] Animate volume destruction
  (bind _returnvalue (`PrimitiveComponent.CreateDynamicMaterialInstance` (`self.Volume`) 0 "/Game/StarterContent/Materials/M_Glass_Inst.M_Glass_Inst"))
  (bind (_direction _alpha) (`Timeline|BoxShrink` :!via `PlayFromStart`)
    (:`Update`
      (`self.SetActorScale3D` (`KismetMathLibrary.VLerp` (`self.Scale`) (0.0 0.0 0.0) _alpha))
      (`MaterialInstanceDynamic.SetVectorParameterValue` _returnvalue "ColorGlass" (`KismetMathLibrary.LinearColorLerp` (struct :`G` 5.7e-05 :`B` 0.098689 :`A` 1.0) (struct :`R` 1.0 :`G` 1.0 :`B` 1.0 :`A` 1.0) _alpha))
      (set `PostProcessComponent.BlendWeight` (`KismetMathLibrary.Lerp` 1.0 0.0 _alpha) (`self.PostProcess1`)))
    (:`Finished`
      (`self.K2_DestroyActor`))))

(fn `Transition`
  (params (DeltaSeconds :type "Float (double-precision)") (TransitionFrom :type "Float (double-precision)") (TransitionTo :type "Float (double-precision)") (TransitionAlpha :type "Float (double-precision)") (TransitionTime :type "Float (double-precision)"))
  (returns (Time :type "Float (double-precision)") (Alpha :type "Float (double-precision)"))
  (locals (From :type "Float (double-precision)") (To :type "Float (double-precision)") (AlphaTime :type "Float (double-precision)") (TransitionTimeLocal :type "Float (double-precision)") (NewTime :type "Float (double-precision)"))
  (bind _to (`local.To`))
  (bind _transitiontimelocal (`local.TransitionTimeLocal`))
  (bind _alphatime (`local.AlphaTime`))
  ;[1 1 1] Calculate new game speed
  (set `local.From` TransitionFrom)
  (set `local.To` TransitionTo)
  (set `local.AlphaTime` TransitionAlpha)
  (set `local.TransitionTimeLocal` TransitionTime)
  (if (== _transitiontimelocal 0.0)
    (return (`local.NewTime`) (`local.AlphaTime`))
    (else
      (`|ExecutionSequence`
        (:`then_0`
          ;[1 1 1] Calculate first alpha value for ease function (if we start calculations when game speed is between slomo and normal speed values)
          (if (`self.CalcAlphaTime`)
            (set `local.AlphaTime` (/ (- (`self.Last Slomo Value`) (`local.From`)) (- (`local.To`) (`local.From`))))
            (set `self.CalcAlphaTime` false)))
        (:`then_1`
          (set `local.AlphaTime` (+ _alphatime (/ (/ DeltaSeconds (`GameplayStatics.GetGlobalTimeDilation`)) _transitiontimelocal)))
          (if (>= _alphatime 1.0)
            (set `self.bTransitionCompleted` true)
            (set `local.NewTime` _to)
            (else
              (set `local.NewTime` (`|EaseFunction` "EaseInOut" (`local.AlphaTime`) (`local.From`) _to))))
          (return (`local.NewTime`) (`local.AlphaTime`)))))))

(fn `UserConstructionScript`
  (`TextRenderComponent.K2_SetText` (`self.TextRender1`) (`KismetTextLibrary.Conv_StringToText` (`KismetStringLibrary.Conv_IntToString` (`self.NumberOfActions`))))
  (set `self.Scale` (`self.GetActorScale3D`)))