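; Character gun weapon that, on its base action, fires a projectile from the mesh's Projectile socket along the pawn's control rotation.
; SpawnProjectile adds a small muzzle explosion and sets mutual move-ignore between the projectile and the pawn's capsule to prevent self-hits.
; A colored beam emitter attached to the projectile targets the muzzle point, forming a trail.
; Each shot also ejects a shell with randomized velocity and spin.
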(event `self.PrivateBaseAction`
  (params (inPawn :type "Pawn Object Reference"))
  (`parent.PrivateBaseAction` inPawn)
  (`self.SpawnProjectile` inPawn (`KismetMathLibrary.MakeTransform` (`SceneComponent.GetSocketLocation` (`self.SkeletalMeshComponent`) "Projectile") (`Pawn.GetControlRotation` inPawn)))
  ;[1 1 1] Spawn shell
  (bind _returnvalue (`|SpawnActorFromClass` "/Game/Blueprints/UCShell.UCShell_C" (`KismetMathLibrary.MakeTransform` (`self.K2_GetActorLocation`) (`self.K2_GetActorRotation`) (0.2 0.2 0.2)) "AlwaysSpawn" "OverrideRootScale"))
  (set `MovementComponent.Velocity` (+ (* (`KismetMathLibrary.GetUpVector` (struct)) (+ (`self.UpShellVelocityMultiplier`) (`KismetMathLibrary.RandomFloatInRange` -100.0 100.0))) (* (`KismetMathLibrary.GetRightVector` (`self.K2_GetActorRotation`)) (+ (`self.RightShellVelocityMultiplier`) (`KismetMathLibrary.RandomFloatInRange` -100.0 100.0))) (* (`KismetMathLibrary.GetForwardVector` (`self.K2_GetActorRotation`)) (`KismetMathLibrary.RandomFloatInRange` -50.0 50.0))) (`/Game/Blueprints/UCShell.ShellMovementComponent` _returnvalue))
  (set `RotatingMovementComponent.RotationRate` (* (`KismetMathLibrary.RandomRotator` false) 3.0) (`/Game/Blueprints/UCShell.ShellRotationComponent` _returnvalue)))

(fn `SpawnProjectile`
  (params (inPawn :type "Pawn Object Reference") (inTransform :type "Transform Structure"))
  (bind _location (.location inTransform))
  (bind _returnvalue (`GameplayStatics.SpawnEmitterAtLocation` "/Game/StarterContent/Particles/P_Explosion.P_Explosion" _location))
  (`SceneComponent.SetRelativeScale3D` _returnvalue (0.1 0.1 0.1))
  (bind _returnvalue_2 (`|SpawnActorFromClass` "/Game/Blueprints/UCProjectile2.UCProjectile2_C" inTransform "AdjustIfPossibleButDontSpawnIfColliding" "OverrideRootScale")) ; Spawn projectile
  ;[1 1 1] Disable self hit
  (`PrimitiveComponent.IgnoreActorWhenMoving` (`/Game/Blueprints/UCProjectile2.CollisionComponent` _returnvalue_2) inPawn true)
  (bind _ascapsule_collision (cast `CapsuleComponent` (`self.K2_GetRootComponent` inPawn)))
  (`PrimitiveComponent.IgnoreActorWhenMoving` _ascapsule_collision _returnvalue_2 true)
  (bind _returnvalue_3 (`GameplayStatics.SpawnEmitterAttached` "/Game/Particles/BeamParticle.BeamParticle" (`/Game/Blueprints/UCProjectile2.CollisionComponent` _returnvalue_2)))
  (`ParticleSystemComponent.SetVectorParameter` _returnvalue_3 "InitialColor" (`self.InitialBeamColor`))
  (`ParticleSystemComponent.SetBeamTargetPoint` _returnvalue_3 0 _location 0))

(fn `UserConstructionScript`
  (`parent.UserConstructionScript`))