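; Enemy bot character that patrols waypoints, hunts the player and fires a socket-attached gun through a Shoot event meant for AnimNotify calls.
; An eye trace, detection box and countdown pick Patrol, Suspicious, Chase or Attack on Tick, setting speed and material color.
; A looping timer trace finds the target for turning and line-of-sight checks.
; Stabs and bullets reduce health, spawn blood and trigger impulse-driven ragdoll, then destruction.
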(event `self.ReceiveBeginPlay`
  (bind _herotpp2 (`self.HeroTPP2`))
  ;[1 1 1] BeginPlay
  (`KismetSystemLibrary.Delay` 0.5)
  (`KismetSystemLibrary.K2_SetTimer` self "CheckForPlayer" 0.1 true)
  ;[1 1 1] Spawn weapon
  (bind _returnvalue (`|SpawnActorFromClass` "/Game/Blueprints/UCWeapon_EnemyBotGun.UCWeapon_EnemyBotGun_C" (`SceneComponent.GetSocketTransform` _herotpp2 "b_Gun" "RTS_World") "AdjustIfPossibleButDontSpawnIfColliding" "OverrideRootScale"))
  (set `self.Weapon` _returnvalue)
  (`self.K2_AttachRootComponentTo` _returnvalue _herotpp2 "b_Gun" "KeepWorldPosition" true))

(event `OnStabbed`
  (params (ImpactLocation :type "Vector Structure") (ImpactNormal :type "Vector Structure") (BoneName :type Name))
  (bind _herotpp2 (`self.HeroTPP2`))
  (bind _herotpp2_2 (`self.HeroTPP2`))
  ;[1 1 1] Called when player stabs me. Knife deals 2 damage! Always spawn particle blood effect and If it kills me, enable ragdoll and add impulse
  (`KismetSystemLibrary.Delay` 0.08)
  (set `self.HitPoints` (- (`self.HitPoints`) 2))
  (`GameplayStatics.SpawnEmitterAtLocation` "/Game/Particles/P_body_bullet_impact.P_body_bullet_impact" ImpactLocation (`KismetMathLibrary.Conv_VectorToRotator` ImpactNormal))
  (`AudioComponent.Play` (`self.BotHitAudioComp`) 0.0)
  (if (not (> (`self.HitPoints`) 0))
    (`PrimitiveComponent.SetSimulatePhysics` (`self.HeroTPP2`) true)
    (`SkeletalMeshComponent.SetAllBodiesBelowSimulatePhysics` _herotpp2 (`SkinnedMeshComponent.GetBoneName` _herotpp2 1) true true)
    (`PrimitiveComponent.AddImpulseAtLocation` _herotpp2 (* ImpactNormal -7500.0) ImpactLocation BoneName)
    ;[1 1 1] OnHit (by bullet). Always reduce health and spawn blood particle, if the shot was lethal, enable ragdoll, add impulse and start dissolve material sequence. When Material is invisible disable collision and destroy actor
    (`|ExecutionSequence` :!label _label
      (:`then_0`
        (`KismetSystemLibrary.Delay` 2.2)
        (`ActorComponent.K2_DestroyComponent` (`self.CapsuleComponent`))
        (`self.SetActorHiddenInGame` true)
        (`self.SetActorEnableCollision` false)
        (`SkeletalMeshComponent.SetAllBodiesBelowSimulatePhysics` _herotpp2_2 (`SkinnedMeshComponent.GetBoneName` _herotpp2_2 1) false true)
        (`KismetSystemLibrary.K2_SetTimer` self "CheckForPlayer")
        (`self.K2_DestroyActor`))
      (:`then_1`
        (`self.Closegate`)))))

(event `Shoot`
  (bind _targetactor (`self.TargetActor`))
  ;[1 1 1] Shoot (this is called from AnimBlueprint only using AnimNotify!)
  ;;[1 1 1] Shoot only if my target is still valid and if I'm alive
  (if (!= _targetactor null)
    (if (> (`self.HitPoints`) 0)
      (`/Game/Blueprints/UCWeapon_EnemyBotGun.BotShot` (`self.Weapon`) _targetactor self)
      ;[1 1 1] Switch On Alert Mode
      (`self.ChangeSpeed` (`self.AttackSpeed`) :!label _label_2)
      (`self.ChangeColor` (struct :`R` 1.0 :`A` 1.0))
      (`self.LookForSuspect`)
      (`self.Chase`)
      (if (`self.IsInView`)
        (`|ExecutionSequence`
          (:`then_1`
            (bind _distance (`self.GetDistanceToPlayer`))
            (`/Engine/EditorBlueprintResources/StandardMacros.CompareFloat` _distance (`self.StopMovementDistance`)
              (:`>`
                (`self.Chase`))
              (:`==`
                (`MovementComponent.StopMovementImmediately` :!label _label_3))
              (:`<`
                (goto _label_3)))))))))

(event `Closegate`
  (bind _herotpp2 (`self.HeroTPP2`))
  ;[1 1 1] OnHit (by bullet). Always reduce health and spawn blood particle, if the shot was lethal, enable ragdoll, add impulse and start dissolve material sequence. When Material is invisible disable collision and destroy actor
  (goto _label_4 :!via `Close`))

(event `self.ReceiveHit`
  (params (MyComp :type "PrimitiveComponent Object Reference") (Other :type "Actor Object Reference") (OtherComp :type "PrimitiveComponent Object Reference") (bSelfMoved :type Boolean) (HitLocation :type "Vector Structure") (HitNormal :type "Vector Structure") (NormalImpulse :type "Vector Structure") (Hit :type "HitResult Structure (by ref)"))
  (bind (_bblockinghit _binitialoverlap _time _location _impactpoint _normal _impactnormal _physmat _hitactor _hitcomponent _hitbonename) (`GameplayStatics.BreakHitResult` Hit))
  (bind _herotpp2 (`self.HeroTPP2`))
  ;[1 1 1] OnHit (by bullet). Always reduce health and spawn blood particle, if the shot was lethal, enable ragdoll, add impulse and start dissolve material sequence. When Material is invisible disable collision and destroy actor
  ;[1 1 1] Detection Precess
  (`|ExecutionSequence`
    (:`then_0`
      (cast `/Game/Blueprints/MyCharacter` Other)
      (set `self.IsInView` true)
      (set `self.DetectionDelayTemp` (`self.DetectionDelay`)))
    (:`then_1`
      (`/Engine/EditorBlueprintResources/StandardMacros.Gate` false :!label _label_4
        (:`Exit`
          (cast `/Game/Blueprints/UCProjectile2` Other)
          (`|ExecutionSequence`
            (:`then_0`
              (set `self.HitPoints` (- (`self.HitPoints`) 1))
              (if (not (> (`self.HitPoints`) 0))
                (`KismetSystemLibrary.K2_SetTimer` self "CheckForPlayer")
                (`PrimitiveComponent.SetSimulatePhysics` (`self.HeroTPP2`) true)
                (`SkeletalMeshComponent.SetAllBodiesBelowSimulatePhysics` _herotpp2 (`SkinnedMeshComponent.GetBoneName` _herotpp2 1) true true)
                (`PrimitiveComponent.AddImpulseAtLocation` _herotpp2 (* _impactnormal -7500.0) _impactpoint _hitbonename)
                (goto _label)))
            (:`then_1`
              (`GameplayStatics.SpawnEmitterAtLocation` "/Game/Particles/P_body_bullet_impact.P_body_bullet_impact" HitLocation (`KismetMathLibrary.Conv_VectorToRotator` HitNormal)))))))))

(event `self.DetectionArea.OnComponentBeginOverlap`
  (params (OverlappedComponent :type "PrimitiveComponent Object Reference") (OtherActor :type "Actor Object Reference") (OtherComp :type "PrimitiveComponent Object Reference") (OtherBodyIndex :type Integer) (bFromSweep :type Boolean) (SweepResult :type "HitResult Structure (by ref)"))
  ;[1 1 1] Detection Precess
  (bind _asmy_character (cast `/Game/Blueprints/MyCharacter` OtherActor))
  (if (`/Game/Blueprints/MyCharacter.IsDead` _asmy_character)
    (set `self.IsSupecious` false)
    (else
      (set `self.IsSupecious` true))))

(event `DebugEvent`
  (params (Debug :type Boolean))
  ;[1 1 1] Detection Area
  (if Debug
    (`SceneComponent.SetHiddenInGame` (`self.DetectionArea`) false false)
    (set `self.TraceDebug` "ForOneFrame")
    (for _array_element (`self.WayPoints`)
      (`KismetSystemLibrary.DrawDebugSphere` (`self.K2_GetActorLocation` _array_element) 30.0 18 (struct :`G` 1.0 :`B` 0.266635 :`A` 1.0) 50000.0))
    (else
      (`SceneComponent.SetHiddenInGame` (`self.DetectionArea`) true false)
      (set `self.TraceDebug` "None")
      (`KismetSystemLibrary.FlushDebugStrings`)
      (`KismetSystemLibrary.FlushPersistentDebugLines`))))

(event `self.DetectionArea.OnComponentEndOverlap`
  (params (OverlappedComponent :type "PrimitiveComponent Object Reference") (OtherActor :type "Actor Object Reference") (OtherComp :type "PrimitiveComponent Object Reference") (OtherBodyIndex :type Integer))
  ;[1 1 1] Detection Precess
  (cast `/Game/Blueprints/MyCharacter` OtherActor)
  (set `self.IsSupecious` false))

(event `PlayerDetectedEvent`
  ;[1 1 1] PlayerDetectedEvent
  (set `self.IsInView` true)
  (set `self.DetectionDelayTemp` (`self.DetectionDelay`)))

(event `self.ReceiveTick`
  (params (DeltaSeconds :type "Float (single-precision)"))
  (bind _yaw (.yaw (`self.K2_GetActorRotation`)))
  (bind _yaw_2 (.yaw (`self.DesiredRotation`)))
  ;[1 1 1] Tick
  (`|ExecutionSequence`
    (:`then_0`
      ;[1 1 1] Detection Precess
      (`self.EyesTrace`))
    (:`then_1`
      ;[1 1 1] Define AlertMode
      (`/Engine/EditorBlueprintResources/StandardMacros.CompareFloat` (`self.DetectionDelayTemp`)
        (:`>`
          (set `self.DetectionDelayTemp` (- (`self.DetectionDelayTemp`) (`GameplayStatics.GetWorldDeltaSeconds`)))
          (bind _distance (`self.GetDistanceToPlayer`))
          (`/Engine/EditorBlueprintResources/StandardMacros.CompareFloat` _distance (`self.AttackDistance`)
            (:`>`
              (set `self.AlertMode` "NewEnumerator1"))
            (:`==`
              (set `self.AlertMode` "NewEnumerator0" :!label _label_5))
            (:`<`
              (goto _label_5))))
        (:`==`
          (if (`self.IsSupecious`) :!label _label_6
            (set `self.AlertMode` "NewEnumerator2")
            (else
              (set `self.AlertMode` "NewEnumerator3"))))
        (:`<`
          (goto _label_6))))
    (:`then_2`
      ;[1 1 1] Switch On Alert Mode
      (switch `/Game/Blueprints/AlertMode` (`self.AlertMode`)
        (:`NewEnumerator0`
          (goto _label_2))
        (:`NewEnumerator1`
          (`self.ChangeSpeed` (`self.ChaseSpeed`))
          (`self.ChangeColor` (struct :`R` 1.0 :`A` 1.0))
          (`self.LookForSuspect`)
          (`self.Chase`))
        (:`NewEnumerator2`
          (`self.ChangeSpeed` (`self.SuspeciousSpeed`))
          (`self.ChangeColor` (struct :`R` 1.0 :`G` 0.452495 :`A` 1.0))
          (`self.LookForSuspect`)
          ;[1 1 1] Patrolling
          (if (<= (`self.GetDistanceTo` (`KismetArrayLibrary.Array_Get` (`self.WayPoints`) (`self.CurrentPoint`))) 200.0) :!label _label_7
            (if (>= (`self.CurrentPoint`) (`KismetArrayLibrary.Array_Length` (`self.WayPoints`)))
              (set `self.CurrentPoint` 0)
              (else
                (set `self.CurrentPoint` (+ (`self.CurrentPoint`) 1))))
            (else
              (`NavigationSystem.SimpleMoveToActor` (`self.GetController`) (`KismetArrayLibrary.Array_Get` (`self.WayPoints`) (`self.CurrentPoint`))))))
        (:`NewEnumerator3`
          (`self.ChangeSpeed` (`self.PatrolSpeed`))
          (`self.ChangeColor` (struct :`R` 0.075141 :`G` 0.805 :`A` 1.0))
          (`self.ResetEyesRotation`)
          (`KismetSystemLibrary.Delay` 4.2)
          (goto _label_7))))
    (:`then_4`
      ;[1 1 1] Tick
      ;;[1 1 1] Only check further if I'm alive
      (if (> (`self.HitPoints`) 0)
        (if (or (!= _yaw _yaw_2) (== _yaw_2 _yaw))
          (if (!= (`self.TargetActor`) null)
            (set `self.bLockTimer` true)
            (`self.K2_SetActorRotation` (`KismetMathLibrary.RLerp` (`self.K2_GetActorRotation`) (`KismetMathLibrary.MakeRotator` 0.0 0.0 _yaw_2) (* DeltaSeconds (`self.RotationRate`)) true))
            (set `self.bHasLOS` (> (`KismetMathLibrary.Dot_VectorVector` (`KismetMathLibrary.Normal` (`KismetMathLibrary.Conv_RotatorToVector` (`self.K2_GetActorRotation`))) (`KismetMathLibrary.Normal` (`KismetMathLibrary.GetDirectionUnitVector` (`self.K2_GetActorLocation`) (`self.K2_GetActorLocation` (`self.TargetActor`))))) 0.85))
            (set `self.bLockTimer` false)
            (else
              (set `self.bHasLOS` false :!label _label_8)
              (set `self.bLockTimer` false)))
          (else
            (goto _label_8)))
        (else
          (goto _label_8))))))

(fn `ChangeColor`
  (params (NewColor :type "LinearColor Structure"))
  (bind _materialinstance (`self.MaterialInstance`))
  (`MaterialInstanceDynamic.SetVectorParameterValue` _materialinstance "Color" NewColor)
  (`PrimitiveComponent.SetMaterial` (`self.HeroTPP2`) 0 _materialinstance))

(fn `ChangeSpeed`
  (params (NewSpeed :type "Float (double-precision)"))
  (set `CharacterMovementComponent.MaxWalkSpeed` (`KismetMathLibrary.Lerp` NewSpeed (`CharacterMovementComponent.MaxWalkSpeed` (`self.CharacterMovement`)) 0.85) (`self.CharacterMovement`)))

(fn `Chase`
  (`NavigationSystem.SimpleMoveToActor` (`self.GetController`) (`GameplayStatics.GetPlayerPawn` 0)))

(fn `CheckForPlayer`
  (bind _returnvalue (`GameplayStatics.GetPlayerCharacter` 0))
  (bind _asmy_character (cast `/Game/Blueprints/MyCharacter` _returnvalue))
  (bind _outhit (`KismetSystemLibrary.LineTraceSingle` (.location (`SceneComponent.GetSocketTransform` (`self.HeroTPP2`) "headSocket" "RTS_World")) (+ (`self.K2_GetActorLocation` _returnvalue) (`SceneComponent.RelativeLocation` (`/Game/Blueprints/MyCharacter.FirstPersonCamera` _asmy_character))) "TraceTypeQuery2"))
  (bind (_bblockinghit _binitialoverlap _time _location _impactpoint _normal _impactnormal _physmat _hitactor) (`GameplayStatics.BreakHitResult` _outhit))
  (if (!= _hitactor null)
    (if (== _hitactor _returnvalue)
      (if (< (`self.GetDistanceTo` _hitactor) (`self.Range`))
        (set `self.DesiredRotation` (`KismetMathLibrary.FindLookAtRotation` (`self.K2_GetActorLocation`) (`self.K2_GetActorLocation` _hitactor)))
        (set `self.TargetActor` _hitactor)
        (else
          (if (not (`self.bLockTimer`)) :!label _label
            (set `self.TargetActor` null))))
      (else
        (goto _label)))))

(fn `EyesTrace`
  (bind _eyes (`self.Eyes`))
  (bind _returnvalue (`SceneComponent.K2_GetComponentLocation` _eyes))
  (bind _outhit (`KismetSystemLibrary.LineTraceSingle` :`Start` _returnvalue :`End` (+ _returnvalue (* (`SceneComponent.GetForwardVector` _eyes) (`self.FieldOfView`))) :`TraceChannel` "TraceTypeQuery1" :`DrawDebugType` (`self.TraceDebug`)))
  (bind _asmy_character (cast `/Game/Blueprints/MyCharacter` (`.HitActor` (`GameplayStatics.BreakHitResult` _outhit)))
    (:`then`
      (if (`/Game/Blueprints/MyCharacter.IsDead` _asmy_character)
        (set `self.DetectionDelayTemp` 0.0)
        (else
          (set `self.IsInView` true)
          (set `self.DetectionDelayTemp` (`self.DetectionDelay`)))))
    (:`CastFailed`
      (set `self.IsInView` false))))

(fn `GetDistanceToPlayer`
  (returns (Distance :type "Float (double-precision)"))
  (return (`self.GetDistanceTo` (`GameplayStatics.GetPlayerPawn` 0))))

(fn `LookForSuspect`
  (bind _eyes (`self.Eyes`))
  (`SceneComponent.K2_SetWorldRotation` _eyes (`KismetMathLibrary.FindLookAtRotation` (`SceneComponent.K2_GetComponentLocation` _eyes) (`self.K2_GetActorLocation` (`GameplayStatics.GetPlayerPawn` 0))) true false))

(fn `ResetEyesRotation`
  (`SceneComponent.K2_SetRelativeRotation` :`self` (`self.Eyes`) :`bSweep` true))

(fn `UserConstructionScript`
  (bind _detectionarea (`self.DetectionArea`))
  (bind _herotpp2 (`self.HeroTPP2`))
  (`|ExecutionSequence`
    (:`then_0`
      (`SceneComponent.K2_SetRelativeLocation` _detectionarea (`self.DetectionAreaRelativeLocation`) false false)
      (`BoxComponent.SetBoxExtent` _detectionarea (`self.DetectionAreaScale`) true)
      (bind _returnvalue (`PrimitiveComponent.CreateDynamicMaterialInstance` (`self.HeroTPP2`) 0 "/Game/Materials/Enemy_Material.Enemy_Material"))
      (set `self.MaterialInstance` _returnvalue))
    (:`then_1`
      (bind _returnvalue_2 (`PrimitiveComponent.CreateDynamicMaterialInstance` _herotpp2 0 "/Game/Materials/M_TestMat.M_TestMat"))
      (set `self.MatInst` _returnvalue_2)
      (`PrimitiveComponent.SetMaterial` _herotpp2 0 (`self.MatInst`)))))