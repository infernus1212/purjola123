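; Coin is a collectible pickup that awards the player a point when MyCharacter overlaps its Collision component.
; A RedCoin flag swaps the Root material at BeginPlay and routes the point to IncomingRedPoints instead of IncomingPoints on the character.
; On pickup it plays the coin sound at the world origin rather than at its own location, then destroys itself.
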(event `self.ReceiveBeginPlay`
  (if (`self.RedCoin`)
    (`PrimitiveComponent.SetMaterial` (`self.Root`) 0 "/Game/Assets/Materials/CoinMat2.CoinMat2")))

(event `self.Collision.OnComponentBeginOverlap`
  (params (OverlappedComponent :type "PrimitiveComponent Object Reference") (OtherActor :type "Actor Object Reference") (OtherComp :type "PrimitiveComponent Object Reference") (OtherBodyIndex :type Integer) (bFromSweep :type Boolean) (SweepResult :type "HitResult Structure (by ref)"))
  (bind _asmy_character (cast `/Game/Blueprints/MyCharacter` OtherActor))
  (if (`self.RedCoin`)
    (`/Game/Blueprints/MyCharacter.IncomingRedPoints` _asmy_character 1)
    (else
      (`/Game/Blueprints/MyCharacter.IncomingPoints` _asmy_character 1)))
  (`GameplayStatics.PlaySoundAtLocation` "/Game/Assets/Audio/Swinger_CoinSound_Cue.Swinger_CoinSound_Cue")
  (`self.K2_DestroyActor`))

(fn `UserConstructionScript`)